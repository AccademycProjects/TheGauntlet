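; BP_Lever is an interactable lever actor that shows a two-state on/off position.
; A Toggle component holds the state, and its on and off delegates snap the Pivot's relative rotation to AnimRotation or its negation.
; BeginPlay applies the same rotation from the current Toggle state so the lever starts in the matching pose.
; Interaction prompt visibility changes show or hide BPInteractionWidget.
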(event OnToggleonDelegate(Toggle)
  (params (ToggleComponent :type Toggle%20Component%20Object%20Reference))
  (Transformation|SetRelativeRotation (Variables|Default|GetPivot) (Variables|Default|GetAnimRotation) false false))

(event OnToggleOffDelegate(Toggle)
  (params (ToggleComponent :type Toggle%20Component%20Object%20Reference))
  (Transformation|SetRelativeRotation (Variables|Default|GetPivot) (* (Variables|Default|GetAnimRotation) (Math|Float|MakeLiteralFloat -1.0)) false false))

(event EventBeginPlay
  (bind _pivot (Variables|Default|GetPivot))
  (bind _animrotation (Variables|Default|GetAnimRotation))
  (if (Class|ToggleComponent|Ison (Variables|Default|GetToggle))
    (Transformation|SetRelativeRotation _pivot _animrotation false false)
    (else
      (Transformation|SetRelativeRotation _pivot (* _animrotation (Math|Float|MakeLiteralFloat -1.0)) false false))))

(event Collision|EventActorBeginOverlap
  (params (OtherActor :type Actor%20Object%20Reference)))

(event EventTick
  (params (DeltaSeconds :type Float%20%28single-precision%29)))

(event EventOnInteractionPromptVisibilityChanged
  (params (bVisible :type Boolean))
  (Rendering|SetVisibility (Variables|Default|GetBP_InteractionWidget) bVisible false))

(fn ConstructionScript)